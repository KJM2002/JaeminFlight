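; BP_Rocket is a rocket actor that removes itself through a short life span set on BeginPlay.
; Two events, named as calls from C++ into Blueprint, print debug strings, and the Default one calls its parent implementation first.
; An explosion chain with a Rocket tag check, Niagara effect, sound, damage and destroy is left unconnected, as is a delayed destroy, so neither runs.
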(event `self.ReceiveBeginPlay`
  (`self.SetLifeSpan` 3.0))

(event `self.CallCPPExecuteBP`
  ; 제발 계산하는거 해줘.
  (`KismetSystemLibrary.PrintString` "이건 블프에서 실행됨"))

(event `self.CallCPPExecuteBPDefault`
  (`parent.CallCPPExecuteBPDefault`)
  (`KismetSystemLibrary.PrintString` "이건 기획 시켜"))

(fn `UserConstructionScript`)